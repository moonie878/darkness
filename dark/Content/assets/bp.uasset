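; Coin pickup actor that spins in the world and credits the player when touched.
; Tick rotates the static mesh on roll and pitch by RotSpeed, scaled by delta time.
; When mycharcter overlaps the mesh, the actor calls Addcoins on it, plays a click sound at its location and destroys itself.
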(event `self.StaticMesh.OnComponentBeginOverlap`
  (params (OverlappedComponent :type "PrimitiveComponent Object Reference") (OtherActor :type "Actor Object Reference") (OtherComp :type "PrimitiveComponent Object Reference") (OtherBodyIndex :type Integer) (bFromSweep :type Boolean) (SweepResult :type "HitResult Structure (by ref)"))
  (bind _asmycharcter (cast `/Game/assets/mycharcter` OtherActor))
  (`/Game/assets/mycharcter.addcoins` _asmycharcter)
  (`GameplayStatics.PlaySoundAtLocation` "/Engine/VREditor/Sounds/UI/Click_on_Button.Click_on_Button" (`self.K2_GetActorLocation`))
  (`self.K2_DestroyActor`))

(event `self.ReceiveTick`
  (params (DeltaSeconds :type "Float (single-precision)"))
  (bind _rotspeed (`self.rotSpeed`))
  (`SceneComponent.K2_AddLocalRotation` (`self.StaticMesh`) (* (`KismetMathLibrary.MakeRotator` _rotspeed _rotspeed) DeltaSeconds) false false))

(fn `UserConstructionScript`)